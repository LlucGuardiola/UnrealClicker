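; ActorClicker is the clickable core of a clicker game, turning mesh clicks into spawned SpawnerMesh actors.
; BeginPlay creates the UI and enables mouse clicks, and each click raises the current and total counters.
; Tick refreshes the UI and, at the click threshold, resets the counter and spawns an actor with a back-reference.
; Trigonometry places spawns in expanding vertical XZ rings, each holding 1.25 times the previous count.
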(event `self.ReceiveTick`
  (params (DeltaSeconds :type "Float (single-precision)"))
  ;[0 0.15 0.1492 0.5] Even Tick - Update game logic
  (`self.UpdateUI`)
  (if (>= (`self.CurrentClicks`) (`self.MaxClicks`))
    (`self.SpawnActor`)
    (`self.ResetClicks`)))

(event `self.ReceiveBeginPlay`
  (bind _returnvalue (`GameplayStatics.GetPlayerController` 0))
  ;[0.15 0 0.01183 0.5] Begin Play - Create UI and enable Cursor
  (bind _returnvalue_2 (`|CreateWidget` "/Game/BluePrints/UI.UI_C"))
  (bind _output_get (set `self.UI` _returnvalue_2))
  (`UserWidget.AddToViewport` _output_get 0)
  (set `PlayerController.bShowMouseCursor` true _returnvalue)
  (set `PlayerController.bEnableClickEvents` true _returnvalue))

(event `AddClicks`
  (params (Clicks :type Integer))
  ;[0.15 0.1029 0 0.5] Add Clicks - Increase TotalClicks and CurrentClicks by "X"
  (set `self.CurrentClicks` (+ Clicks (`self.CurrentClicks`)))
  (set `self.TotalClicks` (+ (`self.TotalClicks`) Clicks)))

(event `UpdateUI`
  (bind _ui (`self.UI`))
  ;[0 0.15 0.01337 0.5] Update UI - Change visual values on the UI
  (`/Game/BluePrints/UI.UpdatePoints` _ui (`self.TotalPoints`))
  (`/Game/BluePrints/UI.UpdateClicks` _ui (`self.TotalClicks`))
  (`/Game/BluePrints/UI.UpdateUIBar` _ui (`self.CurrentClicks`)))

(event `ResetClicks`
  ;[0.09787 0.15 0 0.5] Reset Clicks - Reset Clicks counter
  (set `self.CurrentClicks` (- 10 (`self.CurrentClicks`))))

(event `self.StaticMesh.OnClicked`
  (params (TouchedComponent :type "PrimitiveComponent Object Reference") (ButtonPressed :type "Key Structure"))
  ;[0.15 0 0.1295 0.5] On Actor Clicked - Call Add Clicks event
  (`self.AddClicks` (`self.ClicksToAdd`)))

(event `SpawnActor`
  (bind _radius (`self.Radius`))
  ;[0 0.0162 0.15 0.5] Spawn Actor - Create actors surrounding an Initial position
  (set `self.Radius` (+ (`self.BaseRadius`) (* (`self.CurrentRing`) (`self.RadiusSetup`))))
  (bind _output_get (set `self.Angle` (`KismetMathLibrary.Conv_IntToDouble` (* (`self.CurrentIndex`) (/ 360 (`self.ObjectPerRing`))))))
  (bind _output_get_2 (set `self.AngleRad` (`KismetMathLibrary.DegreesToRadians` _output_get)))
  (bind _returnvalue (`|SpawnActorFromClass` "/Game/BluePrints/SpawnerMesh.SpawnerMesh_C" (`KismetMathLibrary.MakeTransform` (+ (`self.K2_GetActorLocation` self) (`KismetMathLibrary.MakeVector` (* (`KismetMathLibrary.Cos` _output_get_2) _radius) 0.0 (* _radius (`KismetMathLibrary.Sin` _output_get_2))))) "Undefined" "MultiplyWithRoot" null null null))
  (`|ExecutionSequence`
    (:`then_0`
      (set `self.CurrentIndex` (+ (`self.CurrentIndex`) 1))
      (if (>= (`self.CurrentIndex`) (`self.ObjectPerRing`))
        (set `self.CurrentIndex` 0)
        (set `self.CurrentRing` (+ (`self.CurrentRing`) 1))
        (set `self.ObjectPerRing` (* (`self.ObjectPerRing`) 1.25))))
    (:`then_1`
      ;;[0.15 0.1219 0 0.5] Variable of SpawnerMesh
      (set `/Game/BluePrints/SpawnerMesh.ActorClicker` self _returnvalue))))

(fn `UserConstructionScript`)